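; BP_KMKPlayer is a player Blueprint that handles key input for desk interaction, camera state and a chatbot UI.
; E alternates server-named calls for a camera flag, whose Server_ events set IsCamera.
; Left mouse toggles the desk's KMK_PlayerMouse ray, also creating WBP_ChatBotMain without displaying it here.
; Key 1 passes the third-person camera to KMK_DeskComponent for switching, while C displays WBP_ChatBot with a cursor.
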(event Custom|Server_IsCamera
  (Variables|Default|SetIsCamera true))

(event Custom|Server_IsNotCamera
  (Variables|Default|SetIsCamera false))

(event EventBeginPlay)

(event Collision|EventActorBeginOverlap
  (params (OtherActor :type Actor%20Object%20Reference)))

(event EventTick
  (params (DeltaSeconds :type Float%20%28single-precision%29)))

(event Input|MouseEvents|LeftMouseButton
  (params (Key :type Key%20Structure :default "None"))
  (bind _interactioncomp (Variables|Default|GetinteractionComp))
  (bind _deskactor (Variables|/Script/Alchemist.PlayerInteractionComponent|GetDeskActor _interactioncomp))
  (bind _returnvalue (Actor|GetComponentbyClass _deskactor "/Script/Alchemist.KMK_PlayerMouse"))
  (:Pressed
    (Utilities|IsValid _deskactor
      (:Is%20Valid
        (Variables|/Script/Alchemist.KMK_PlayerMouse|SetIsRay _returnvalue true)
        (UserInterface|CreateWidget "/Game/Project/KMK/UI/WBP_ChatBotMain.WBP_ChatBotMain_C"))))
  (:Released
    (Utilities|IsValid _deskactor
      (:Is%20Valid
        (Variables|/Script/Alchemist.KMK_PlayerMouse|SetIsRay _returnvalue false)))))

(event Input|KeyboardEvents|E
  (params (Key :type Key%20Structure :default "None"))
  (:Pressed
    (Utilities|FlowControl|FlipFlop
      (:A
        (CallFunction|ServerIsCamera))
      (:B
        (CallFunction|ServerIsNotCamera)))))

(event Input|KeyboardEvents|C
  (params (Key :type Key%20Structure :default "None"))
  (bind _returnvalue (Game|GetPlayerController 0))
  (:Pressed
    (bind _returnvalue_2 (UserInterface|CreateWidget "/Game/Project/KMK/UI/WBP_ChatBot.WBP_ChatBot_C"))
    (UserInterface|Viewport|AddtoViewport _returnvalue_2 0)
    (if (Pawn|IsLocalPlayerController _returnvalue)
      (Variables|/Script/Engine.PlayerController|SetbShowMouseCursor _returnvalue true))))

(event Input|KeyboardEvents|1
  (params (Key :type Key%20Structure :default "None"))
  (bind _interactioncomp (Variables|Default|GetinteractionComp))
  (bind _deskactor (Variables|/Script/Alchemist.PlayerInteractionComponent|GetDeskActor _interactioncomp))
  (bind _returnvalue (Actor|GetComponentbyClass _deskactor "/Script/Alchemist.KMK_DeskComponent"))
  (:Pressed
    (Variables|/Script/Alchemist.KMK_DeskComponent|SetPlayerCamera _returnvalue (Variables|Default|GetCameraCompThird))
    (Class|KMKDeskComponent|ChangeMyCamera _returnvalue false)))

(fn ConstructionScript)