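; BP_NewElement is an element actor that rises to a fixed height.
; While IsUp on KMKElementGameActor is false, Tick moves it along its up vector at Speed without sweeping, then holds world Z at the height cap.
; The node that would set IsUp true is unconnected, so this graph never ends the rise check itself.
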(event EventBeginPlay)

(event Collision|EventActorBeginOverlap
  (params (OtherActor :type Actor%20Object%20Reference)))

(event EventTick
  (params (DeltaSeconds :type Float%20%28single-precision%29))
  (bind _returnvalue (Transformation|GetActorLocation))
  (if (not (Variables|/Script/Alchemist.KMK_ElementGameActor|GetisUp (Variables|Default|GetKMK_ElementGameActor)))
    (if (>= (.z (Transformation|GetActorLocation)) 3e+02)
      (Transformation|SetActorLocation (Math|Vector|MakeVector (.x _returnvalue) (.y _returnvalue) 3e+02) false false)
      (else
        (Transformation|SetActorLocation (+ (* DeltaSeconds (Variables|Default|Getspeed) (Transformation|GetActorUpVector)) (Transformation|GetActorLocation)) false false)))))

(fn ConstructionScript)