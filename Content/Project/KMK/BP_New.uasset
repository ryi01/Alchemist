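; Player Blueprint that handles input for camera and jump states, desk widget interaction and chatbot UI.
; On BeginPlay, the local player links "Pot"-tagged actors' grab components to InteractionComp and new mission chatbot widgets.
; E toggles IsCamera and Space sets IsJump through server and client events.
; While IsWidget, left click drives WidgetInteraction and desk raycasting; 1 returns to third-person camera, C opens a chatbot.
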(event Custom|Server_IsCamera
  (Variables|Default|SetIsCamera true))

(event Custom|Client_IsNotCamera
  (Variables|Default|SetIsCamera false))

(event Custom|Server_IsJump
  (Variables|Default|SetIsJump true))

(event Custom|Client_IsCamera
  (Variables|Default|SetIsCamera true))

(event Custom|Server_IsNotCamera
  (Variables|Default|SetIsCamera false))

(event Custom|Client_IsJump
  (Variables|Default|SetIsJump true))

(event EventBeginPlay
  (bind _outactors (Actor|GetAllActorswithTag "Pot"))
  (for _array_element _outactors
    (if (Pawn|IsLocalPlayerController (Game|GetPlayerController 0))
      (bind _returnvalue (UserInterface|CreateWidget "/Game/Project/KMK/UI/WBP_ChatBotMain.WBP_ChatBotMain_C"))
      (Utilities|IsValid (Actor|GetComponentbyClass _array_element "/Script/Alchemist.KMK_GrabActorComp")
        (:Is%20Valid
          (Variables|/Script/Alchemist.PlayerInteractionComponent|SetpotComp (Variables|Default|GetinteractionComp) (Actor|GetComponentbyClass _array_element "/Script/Alchemist.KMK_GrabActorComp"))
          (Variables|/Script/Alchemist.KMK_GrabActorComp|SetmissionWidget (Actor|GetComponentbyClass _array_element "/Script/Alchemist.KMK_GrabActorComp") _returnvalue)
          (UserInterface|Viewport|AddtoViewport _returnvalue 0))))))

(event Collision|EventActorBeginOverlap
  (params (OtherActor :type Actor%20Object%20Reference)))

(event EventTick
  (params (DeltaSeconds :type Float%20%28single-precision%29)))

(event Input|MouseEvents|LeftMouseButton
  (params (Key :type Key%20Structure :default "None"))
  (bind _returnvalue (Game|GetPlayerController 0))
  (bind _interactioncomp (Variables|Default|GetinteractionComp))
  (bind _interactioncomp_2 (Variables|Default|GetinteractionComp))
  (bind _deskactor (Variables|/Script/Alchemist.PlayerInteractionComponent|GetDeskActor _interactioncomp_2))
  (bind _deskactor_2 (Variables|/Script/Alchemist.PlayerInteractionComponent|GetDeskActor _interactioncomp))
  (:Pressed
    (if (Variables|Default|GetisWidget)
      (if (Pawn|IsLocalPlayerController _returnvalue)
        (Variables|/Script/Engine.PlayerController|SetbShowMouseCursor _returnvalue true)
        (Input|SetInputModeGameandUI _returnvalue 0 "DoNotLock" false false)
        (Utilities|IsValid _deskactor
          (:Is%20Valid
            (Variables|/Script/Alchemist.KMK_PlayerMouse|SetIsRay (Actor|GetComponentbyClass _deskactor "/Script/Alchemist.KMK_PlayerMouse") true)
            (Class|WidgetInteractionComponent|PressPointerKey (Variables|Default|GetWidgetInteraction) "LeftMouseButton")
            (UserInterface|CreateWidget "/Game/Project/KMK/UI/WBP_ChatBotMain.WBP_ChatBotMain_C"))))))
  (:Released
    (if (Variables|Default|GetisWidget)
      (Class|WidgetInteractionComponent|ReleasePointerKey (Variables|Default|GetWidgetInteraction) "LeftMouseButton")
      (Utilities|IsValid _deskactor_2
        (:Is%20Valid
          (Variables|/Script/Alchemist.KMK_PlayerMouse|SetIsRay (Actor|GetComponentbyClass _deskactor_2 "/Script/Alchemist.KMK_PlayerMouse") false))))))

(event Input|KeyboardEvents|SpaceBar
  (params (Key :type Key%20Structure :default "None"))
  (:Pressed
    (CallFunction|ServerIsJump)
    (CallFunction|ClientIsJump)))

(event Input|KeyboardEvents|C
  (params (Key :type Key%20Structure :default "None"))
  (bind _returnvalue (Game|GetPlayerController 0))
  (:Pressed
    (bind _returnvalue_2 (UserInterface|CreateWidget "/Game/Project/KMK/UI/WBP_ChatBot.WBP_ChatBot_C"))
    (UserInterface|Viewport|AddtoViewport _returnvalue_2 0)
    (if (Pawn|IsLocalPlayerController _returnvalue)
      (Variables|/Script/Engine.PlayerController|SetbShowMouseCursor _returnvalue true))))

(event Input|KeyboardEvents|E
  (params (Key :type Key%20Structure :default "None"))
  (:Pressed
    (Utilities|FlowControl|FlipFlop
      (:A
        (CallFunction|ServerIsCamera)
        (CallFunction|ClientIsCamera))
      (:B
        (CallFunction|ServerIsNotCamera)
        (CallFunction|ClientIsNotCamera)))))

(event Input|KeyboardEvents|1
  (params (Key :type Key%20Structure :default "None"))
  (bind _returnvalue (Game|GetPlayerController 0))
  (bind _interactioncomp (Variables|Default|GetinteractionComp))
  (bind _deskactor (Variables|/Script/Alchemist.PlayerInteractionComponent|GetDeskActor _interactioncomp))
  (bind _returnvalue_2 (Actor|GetComponentbyClass _deskactor "/Script/Alchemist.KMK_DeskComponent"))
  (:Pressed
    (Variables|Default|SetisWidget false)
    (Variables|/Script/Alchemist.KMK_DeskComponent|SetPlayerCamera _returnvalue_2 (Variables|Default|GetCameraCompThird))
    (Class|KMKDeskComponent|ChangeMyCamera _returnvalue_2 false)
    (if (Pawn|IsLocalPlayerController _returnvalue)
      (Variables|/Script/Engine.PlayerController|SetbShowMouseCursor _returnvalue false)
      (Input|SetInputModeGameOnly _returnvalue false))))

(fn ConstructionScript)